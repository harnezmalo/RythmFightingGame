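; Player Blueprint that turns directional input into move commands for the game manager.
; On BeginPlay it caches the BP_GameManager found in the level and adds the IMC_Custom Enhanced Input mapping context to its player controller.
; The forward, backward, up and down actions each set the manager's Direction and a signed Axis value, then share one call to the manager's Move.
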(event `self.ReceiveBeginPlay`
  (`|ExecutionSequence`
    (:`then_0`
      (bind _returnvalue (`GameplayStatics.GetActorOfClass` "/Game/Blueprints/Assets/BP_GameManager.BP_GameManager_C"))
      (set `self.GameManager` _returnvalue))
    (:`then_1`
      (bind _asplayer_controller (cast `PlayerController` (`self.GetController`)))
      (bind _returnvalue_2 (pcsubsystem `EnhancedInputLocalPlayerSubsystem` _asplayer_controller))
      (`/Engine/EditorBlueprintResources/StandardMacros.IsValid` _returnvalue_2
        (:`Is Valid`
          (`EnhancedInputSubsystemInterface.AddMappingContext` _returnvalue_2 "/Game/Blueprints/Mapping/IMC_Custom.IMC_Custom" 0 (struct)))))))

(event `EnhancedInput|/Game/Blueprints/Mapping/Inputs/IA_Forward`
  (params (ActionValue :type Boolean) (ElapsedSeconds :type "Float (double-precision)") (TriggeredSeconds :type "Float (double-precision)") (InputAction :type "InputAction Object Reference" :default "/Game/Blueprints/Mapping/Inputs/IA_Forward.IA_Forward"))
  (bind _gamemanager (`self.GameManager`))
  (:`Triggered`
    (set `/Game/Blueprints/Assets/BP_GameManager.Direction` "NewEnumerator0" _gamemanager)
    (set `self.Axis` 1.0)
    (`/Game/Blueprints/Assets/BP_GameManager.Move` _gamemanager :!label _label)))

(event `EnhancedInput|/Game/Blueprints/Mapping/Inputs/IA_Backward`
  (params (ActionValue :type Boolean) (ElapsedSeconds :type "Float (double-precision)") (TriggeredSeconds :type "Float (double-precision)") (InputAction :type "InputAction Object Reference" :default "/Game/Blueprints/Mapping/Inputs/IA_Backward.IA_Backward"))
  (:`Triggered`
    (set `/Game/Blueprints/Assets/BP_GameManager.Direction` "NewEnumerator1" (`self.GameManager`))
    (set `self.Axis` -1.0)
    (goto _label)))

(event `EnhancedInput|/Game/Blueprints/Mapping/Inputs/IA_Up`
  (params (ActionValue :type Boolean) (ElapsedSeconds :type "Float (double-precision)") (TriggeredSeconds :type "Float (double-precision)") (InputAction :type "InputAction Object Reference" :default "/Game/Blueprints/Mapping/Inputs/IA_Up.IA_Up"))
  (:`Triggered`
    (set `/Game/Blueprints/Assets/BP_GameManager.Direction` "NewEnumerator2" (`self.GameManager`))
    (set `self.Axis` -1.0)
    (goto _label)))

(event `EnhancedInput|/Game/Blueprints/Mapping/Inputs/IA_Down`
  (params (ActionValue :type Boolean) (ElapsedSeconds :type "Float (double-precision)") (TriggeredSeconds :type "Float (double-precision)") (InputAction :type "InputAction Object Reference" :default "/Game/Blueprints/Mapping/Inputs/IA_Down.IA_Down"))
  (:`Triggered`
    (set `/Game/Blueprints/Assets/BP_GameManager.Direction` "NewEnumerator3" (`self.GameManager`))
    (set `self.Axis` 1.0)
    (goto _label)))

(fn `UserConstructionScript`)
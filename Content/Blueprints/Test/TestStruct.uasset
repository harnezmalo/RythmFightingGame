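; Test rhythm-game actor that spawns timing rings (TestAnneau) and moves along a spline on well-timed Space presses.
; A looping timer tracks elapsed time against the TimeStamps DataTable, spawning and queuing a ring roughly 1.5 seconds around each timestamp until rows run out.
; When the first queued ring is Good, Space calls GoodTiming and plays a Timeline advancing the actor a fifth of TestSpline's length.
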(event `self.ReceiveBeginPlay`
  (`self.EnableInput` (`GameplayStatics.GetPlayerController` 0))
  (`self.Anneaux`)
  (bind _returnvalue (`GameplayStatics.GetActorOfClass` "/Game/Blueprints/Test/TestSpline.TestSpline_C"))
  (set `self.SplineObj` _returnvalue))

(event `Anneaux`
  (set `self.TempsPassé` 0.0)
  (set `self.TimeStampNum` 1)
  (bind _returnvalue (`KismetSystemLibrary.K2_SetTimerDelegate` (delegate `Update`) 0.1 true)))

(event `Update`
  (bind _output_get (set `self.TempsPassé` (+ (`self.TempsPassé`) 0.1)))
  (bind _returnvalue (`|GetDataTableRow` (`self.Time Stamps`) (`KismetStringLibrary.Conv_StringToName` (`KismetStringLibrary.Conv_IntToString` (`self.TimeStampNum`))))
    (:`then`
      (if (<= (- (`KismetMathLibrary.Abs` (- (`.TimeStamps_8_F2F1298245217A25CA11829E662FE579` (break `/Game/Blueprints/Structures/Struct_TimeStampsImport` _returnvalue)) _output_get)) 1.5) 0.01)
        (bind _returnvalue_2 (`|SpawnActorFromClass` "/Game/Blueprints/Test/TestAnneau.TestAnneau_C" (`self.GetTransform`) "AlwaysSpawn" "MultiplyWithRoot" null null))
        (set `/Game/Blueprints/Test/TestAnneau.Parent` self _returnvalue_2)
        (`KismetArrayLibrary.Array_Add` (`self.AnneauxArray`) _returnvalue_2)
        (set `self.TimeStampNum` (+ (`self.TimeStampNum`) 1))))
    (:`RowNotFound`
      (`KismetSystemLibrary.K2_ClearAndInvalidateTimerHandle` (stale `Anneaux` _returnvalue))
      (set `self.IsPlaying` false))))

(event `Key|SpaceBar`
  (params (Key :type "Key Structure"))
  (bind _output (`|GetArrayItem` (`self.AnneauxArray`)))
  (bind _spline (`/Game/Blueprints/Test/TestSpline.Spline` (`self.SplineObj`)))
  (bind _returnvalue (`SplineComponent.GetDistanceAlongSplineAtLocation` _spline (`self.K2_GetActorLocation`) "World"))
  (:`Pressed`
    (if (`/Game/Blueprints/Test/TestAnneau.Good` _output)
      (`/Game/Blueprints/Test/TestAnneau.GoodTiming` _output)
      (bind _output_get (set `self.Départ` _returnvalue))
      (bind _output_get_2 (set `self.Arrivée` (+ _returnvalue (* (`SplineComponent.GetSplineLength` _spline) 0.2))))
      (bind (_direction _newtrack_0) (`Timeline|Timeline` :!via `PlayFromStart`)
        (:`Update`
          (`self.K2_SetActorLocation` (`SplineComponent.GetLocationAtDistanceAlongSpline` _spline (`KismetMathLibrary.Lerp` _output_get _output_get_2 _newtrack_0) "World")))))))

(fn `UserConstructionScript`)
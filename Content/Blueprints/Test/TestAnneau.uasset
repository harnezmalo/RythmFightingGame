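; Test ring actor (Anneau) for a timing mechanic, which hovers above BP_Player by following its location every Tick.
; A timeline scales the sphere from BeginPlay and sets a Good flag whenever the scale is at or below a threshold.
; The ring removes itself from the game manager's AnneauxArray and destroys itself when the timeline finishes or GoodTiming is called.
; Disconnected nodes for replaying the ring sequence through the game manager never run.
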(event `self.ReceiveBeginPlay`
  (`GameplayStatics.GetActorOfClass` "/Game/Blueprints/Assets/BP_Spline.BP_Spline_C")
  (set `self.Spline` null)
  (bind _returnvalue (`GameplayStatics.GetActorOfClass` "/Game/Blueprints/Contrôlables/BP_Player.BP_Player_C"))
  (set `self.BP_Player` _returnvalue)
  (bind (_direction _newtrack_0) (`Timeline|Timeline` :!via `PlayFromStart`)
    (:`Update`
      (`SceneComponent.SetRelativeScale3D` (`self.Sphere`) (`KismetMathLibrary.MakeVector` _newtrack_0 _newtrack_0 _newtrack_0))
      (if (<= _newtrack_0 1.68)
        (set `self.Good` true)))
    (:`Finished`
      (`KismetArrayLibrary.Array_RemoveItem` (`/Game/Blueprints/Assets/BP_GameManager.AnneauxArray` (`self.BP_GameManager`)) self)
      (`self.K2_DestroyActor`))))

(event `GoodTiming`
  (`KismetArrayLibrary.Array_RemoveItem` (`/Game/Blueprints/Assets/BP_GameManager.AnneauxArray` (`self.BP_GameManager`)) self)
  (`self.K2_DestroyActor`))

(event `self.ReceiveTick`
  (params (DeltaSeconds :type "Float (single-precision)"))
  (`self.K2_SetActorLocation` (`KismetMathLibrary.MakeVector` (.x (`self.K2_GetActorLocation` (`self.BP_Player`))) (.y (`self.K2_GetActorLocation` (`self.BP_Player`))) (+ (.z (`self.K2_GetActorLocation` (`self.BP_Player`))) 120.0))))

(fn `UserConstructionScript`)
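; BP_Cam is a camera actor that follows BP_Player along the X axis while turning to look at it.
; On BeginPlay it finds the player actor, sets itself as player controller 0's view target and snaps into position.
; Every Tick it copies the player's X, keeps its own Y and Z, and rotates with a look-at rotation toward the player.
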(event `self.ReceiveBeginPlay`
  (bind _returnvalue (`GameplayStatics.GetActorOfClass` "/Game/Blueprints/Contrôlables/BP_Player.BP_Player_C"))
  (set `self.Player` _returnvalue)
  (`PlayerController.SetViewTargetWithBlend` (`GameplayStatics.GetPlayerController` 0) self 0.0 "VTBlend_Linear" 0.0 false)
  (`self.K2_SetActorLocation` (`KismetMathLibrary.MakeVector` (.x (`self.K2_GetActorLocation` (`self.Player`))) (.y (`self.K2_GetActorLocation` self)) (.z (`self.K2_GetActorLocation` self))))
  (`self.K2_SetActorRotation` (`KismetMathLibrary.FindLookAtRotation` (`self.K2_GetActorLocation` self) (`self.K2_GetActorLocation` (`self.Player`)))))

(event `self.ReceiveTick`
  (params (DeltaSeconds :type "Float (single-precision)"))
  (`self.K2_SetActorLocation` (`KismetMathLibrary.MakeVector` (.x (`self.K2_GetActorLocation` (`self.Player`))) (.y (`self.K2_GetActorLocation` self)) (.z (`self.K2_GetActorLocation` self))))
  (`self.K2_SetActorRotation` (`KismetMathLibrary.FindLookAtRotation` (`self.K2_GetActorLocation` self) (`self.K2_GetActorLocation` (`self.Player`)))))

(fn `UserConstructionScript`)
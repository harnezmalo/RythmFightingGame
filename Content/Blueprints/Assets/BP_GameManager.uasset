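; Game manager for a rhythm game where the player moves point to point along splines on timed rings.
; BeginPlay spawns collision at every spline point and places the player on the main spline's start.
; A looping timer reads the TimeStamps table to spawn rings ahead of each beat.
; ToMove sphere-traces camera-relative directions for connected points and shows arrows; Move requires a well-timed ring, then slides the player there via Timeline.
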(event `self.ReceiveBeginPlay`
  (bind _player (`self.Player`))
  (`|ExecutionSequence`
    (:`then_0`
      (bind _outactors (`GameplayStatics.GetAllActorsOfClass` "/Game/Blueprints/Assets/BP_Spline.BP_Spline_C"))
      (for _array_element _outactors
        (bind _spline (`/Game/Blueprints/Assets/BP_Spline.Spline` _array_element))
        (for _index (range (`SplineComponent.GetNumberOfSplinePoints` _spline))
          (`self.Instantiate spline point collision` (`SplineComponent.GetTransformAtSplinePoint` _spline _index "World" false) _array_element _index)
          (bind _returnvalue (`GameplayStatics.GetActorOfClass` "/Game/Blueprints/Assets/BP_Cam.BP_Cam_C"))
          (set `self.Cam` _returnvalue))))
    (:`then_1`
      (bind _outactors_2 (`GameplayStatics.GetAllActorsOfClass` "/Game/Blueprints/Assets/BP_Spline.BP_Spline_C"))
      (for _array_element_2 _outactors_2
        (if (`/Game/Blueprints/Assets/BP_Spline.Main` _array_element_2)
          (set `self.BP_Spline` _array_element_2)))
      (bind _returnvalue_2 (`GameplayStatics.GetActorOfClass` "/Game/Blueprints/Contrôlables/BP_Player.BP_Player_C"))
      (set `self.Player` _returnvalue_2)
      (`self.Anneaux`)
      (`self.K2_SetActorLocation` _player (`KismetMathLibrary.MakeVector` (.x (`SplineComponent.GetLocationAtDistanceAlongSpline` (`/Game/Blueprints/Assets/BP_Spline.Spline` (`self.BP_Spline`)) 0.0 "World")) (.y (`SplineComponent.GetLocationAtDistanceAlongSpline` (`/Game/Blueprints/Assets/BP_Spline.Spline` (`self.BP_Spline`)) 0.0 "World")) (.z (`self.K2_GetActorLocation` _player))) false false))
    (:`then_2`
      (`self.debut`))))

(event `Anneaux`
  (set `self.TempsPassé` 0.0)
  (set `self.TimeStampNum` 1)
  (bind _returnvalue (`KismetSystemLibrary.K2_SetTimerDelegate` (delegate `Update`) 0.1 true)))

(event `Update`
  (bind _output_get (set `self.TempsPassé` (+ (`self.TempsPassé`) 0.1)))
  (bind _returnvalue (`|GetDataTableRow` (`self.Time Stamps`) (`KismetStringLibrary.Conv_StringToName` (`KismetStringLibrary.Conv_IntToString` (`self.TimeStampNum`))))
    (:`then`
      (if (<= (- (`KismetMathLibrary.Abs` (- (`.TimeStamps_8_F2F1298245217A25CA11829E662FE579` (break `/Game/Blueprints/Structures/Struct_TimeStampsImport` _returnvalue)) _output_get)) 1.5) 0.01)
        (bind _returnvalue_2 (`|SpawnActorFromClass` "/Game/Blueprints/Test/TestAnneau.TestAnneau_C" (`KismetMathLibrary.MakeTransform` (`KismetMathLibrary.MakeVector` (.x (.location (`self.GetTransform` (`self.Player`)))) (.y (.location (`self.GetTransform` (`self.Player`)))) (+ (.z (.location (`self.GetTransform` (`self.Player`)))) 120.0)) (.rotation (`self.GetTransform` (`self.Player`))) (.scale (`self.GetTransform` (`self.Player`)))) "AlwaysSpawn" "MultiplyWithRoot" null null))
        (set `/Game/Blueprints/Test/TestAnneau.BP_GameManager` self _returnvalue_2)
        (`KismetArrayLibrary.Array_Add` (`self.AnneauxArray`) _returnvalue_2)
        (set `self.TimeStampNum` (+ (`self.TimeStampNum`) 1))))
    (:`RowNotFound`
      (`KismetSystemLibrary.K2_ClearAndInvalidateTimerHandle` (stale `Anneaux` _returnvalue))
      (set `self.IsPlaying` false))))

(event `debut`
  (`KismetSystemLibrary.Delay` 0.2)
  (`self.ToMove`))

(event `Move`
  (bind _player (`self.Player`))
  (bind _output (`|GetArrayItem` (`self.AnneauxArray`)))
  (bind _spline (`/Game/Blueprints/Assets/BP_Spline.Spline` (`self.BP_Spline`)))
  (`/Engine/EditorBlueprintResources/StandardMacros.IsValid` _output
    (:`Is Valid`
      (if (`/Game/Blueprints/Test/TestAnneau.Good` _output)
        (`self.Destroy Arrows`)
        (`/Game/Blueprints/Test/TestAnneau.GoodTiming` _output)
        (switch `/Game/Blueprints/Structures/Enum_Directions` (`self.Direction`)
          (:`NewEnumerator0`
            (set `self.End Point` (`self.RightPoint`)))
          (:`NewEnumerator1`
            (set `self.End Point` (`self.LeftPoint`)))
          (:`NewEnumerator2`
            (set `self.End Point` (`self.UpPoint`)))
          (:`NewEnumerator3`
            (set `self.End Point` (`self.DownPoint`))))
        (for _array_element (`self.Current Points`)
          (bind _asbp_spline_point_collision (cast `/Game/Blueprints/Assets/BP_SplinePointCollision` _array_element))
          (if (== (`/Game/Blueprints/Assets/BP_SplinePointCollision.Spline` _asbp_spline_point_collision) (`/Game/Blueprints/Assets/BP_SplinePointCollision.Spline` (`self.End Point`)))
            (bind _output_get (set `self.Start Point` _asbp_spline_point_collision))
            (set `self.BP_Spline` (`/Game/Blueprints/Assets/BP_SplinePointCollision.Spline` _output_get))))
        (if (`KismetSystemLibrary.IsValid` (`self.End Point`))
          (bind (_direction _newtrack_2) (`Timeline|Timeline` :!via `PlayFromStart`)
            (:`Update`
              (bind _returnvalue (`KismetMathLibrary.Lerp` (`SplineComponent.GetDistanceAlongSplineAtSplinePoint` (`/Game/Blueprints/Assets/BP_Spline.Spline` (`self.BP_Spline`)) (`/Game/Blueprints/Assets/BP_SplinePointCollision.Indice` (`self.Start Point`))) (`SplineComponent.GetDistanceAlongSplineAtSplinePoint` (`/Game/Blueprints/Assets/BP_Spline.Spline` (`self.BP_Spline`)) (`/Game/Blueprints/Assets/BP_SplinePointCollision.Indice` (`self.End Point`))) _newtrack_2))
              (`self.K2_SetActorLocation` _player (`KismetMathLibrary.MakeVector` (.x (`SplineComponent.GetLocationAtDistanceAlongSpline` _spline _returnvalue "World")) (.y (`SplineComponent.GetLocationAtDistanceAlongSpline` _spline _returnvalue "World")) (.z (`self.K2_GetActorLocation` (`self.Player`)))) false false)
              (`self.K2_SetActorRotation` _player (`KismetMathLibrary.MakeRotator` 0.0 0.0 (.yaw (`KismetMathLibrary.MakeRotFromX` (* (`SplineComponent.GetTangentAtDistanceAlongSpline` _spline _returnvalue "World") (`/Game/Blueprints/Contrôlables/BP_Player.Axis` (`self.Player`)))))) false))
            (:`Finished`
              (`self.ToMove`)))
          (else
            (`self.ToMove`)))))))

(fn `Create Arrows`
  (params (R :type "/Game/Blueprints/Assets/BP_SplinePointCollision Object Reference") (L :type "/Game/Blueprints/Assets/BP_SplinePointCollision Object Reference") (U :type "/Game/Blueprints/Assets/BP_SplinePointCollision Object Reference") (D :type "/Game/Blueprints/Assets/BP_SplinePointCollision Object Reference"))
  (`|ExecutionSequence`
    (:`then_0`
      (`/Engine/EditorBlueprintResources/StandardMacros.IsValid` R
        (:`Is Valid`
          (`|SpawnActorFromClass` "/Game/Blueprints/Assets/BP_Arrow.BP_Arrow_C" (`self.GetTransform` R) "AlwaysSpawn" "MultiplyWithRoot" null null))))
    (:`then_1`
      (`/Engine/EditorBlueprintResources/StandardMacros.IsValid` L
        (:`Is Valid`
          (`|SpawnActorFromClass` "/Game/Blueprints/Assets/BP_Arrow.BP_Arrow_C" (`self.GetTransform` L) "AlwaysSpawn" "MultiplyWithRoot" null null))))
    (:`then_2`
      (`/Engine/EditorBlueprintResources/StandardMacros.IsValid` U
        (:`Is Valid`
          (`|SpawnActorFromClass` "/Game/Blueprints/Assets/BP_Arrow.BP_Arrow_C" (`self.GetTransform` U) "AlwaysSpawn" "MultiplyWithRoot" null null))))
    (:`then_3`
      (`/Engine/EditorBlueprintResources/StandardMacros.IsValid` D
        (:`Is Valid`
          (`|SpawnActorFromClass` "/Game/Blueprints/Assets/BP_Arrow.BP_Arrow_C" (`self.GetTransform` D) "AlwaysSpawn" "MultiplyWithRoot" null null))))))

(fn `Destroy Arrows`
  (bind _outactors (`GameplayStatics.GetAllActorsOfClass` "/Game/Blueprints/Assets/BP_Arrow.BP_Arrow_C"))
  (for _array_element _outactors
    (`self.K2_DestroyActor` _array_element)))

(fn `GetCurrentPoints`
  (returns (CurrentPoints :type "Array of Actor Object Reference") (Splines :type "Array of /Game/Blueprints/Assets/BP_Spline Object Reference"))
  (locals (`Splines Contact` :type "Array of /Game/Blueprints/Assets/BP_Spline Object Reference"))
  (`KismetArrayLibrary.Array_Clear` (`local.Splines Contact`))
  (bind _returnvalue (`GameplayStatics.GetActorOfClass` "/Game/Blueprints/Contrôlables/BP_Player.BP_Player_C"))
  (bind _overlappingactors (`PrimitiveComponent.GetOverlappingActors` (`Character.CapsuleComponent` _returnvalue) "/Game/Blueprints/Assets/BP_SplinePointCollision.BP_SplinePointCollision_C"))
  (for _array_element _overlappingactors
    (bind _asbp_spline_point_collision (cast `/Game/Blueprints/Assets/BP_SplinePointCollision` _array_element))
    (bind _spline (`/Game/Blueprints/Assets/BP_SplinePointCollision.Spline` _asbp_spline_point_collision))
    (if (== (`KismetArrayLibrary.Array_Contains` (`local.Splines Contact`) _spline) false)
      (`KismetArrayLibrary.Array_Add` (`local.Splines Contact`) _spline)))
  (return _overlappingactors (`local.Splines Contact`)))

(fn `GetNextPoints`
  (params (CurrentPoints :type "Array of Actor Object Reference") (Splines :type "Array of /Game/Blueprints/Assets/BP_Spline Object Reference"))
  (returns (Right :type "/Game/Blueprints/Assets/BP_SplinePointCollision Object Reference") (Left :type "/Game/Blueprints/Assets/BP_SplinePointCollision Object Reference") (Up :type "/Game/Blueprints/Assets/BP_SplinePointCollision Object Reference") (Down :type "/Game/Blueprints/Assets/BP_SplinePointCollision Object Reference"))
  (locals (DistRight :type "Float (double-precision)" :default 99999.0) (DistLeft :type "Float (double-precision)" :default 99999.0) (DistUp :type "Float (double-precision)" :default 99999.0) (DistDown :type "Float (double-precision)" :default 99999.0) (R :type "/Game/Blueprints/Assets/BP_SplinePointCollision Object Reference") (L :type "/Game/Blueprints/Assets/BP_SplinePointCollision Object Reference") (U :type "/Game/Blueprints/Assets/BP_SplinePointCollision Object Reference") (D :type "/Game/Blueprints/Assets/BP_SplinePointCollision Object Reference"))
  (bind _returnvalue (`KismetMathLibrary.MakeVector` (.x (`self.K2_GetActorLocation` (`self.Player`))) (.y (`self.K2_GetActorLocation` (`self.Player`)))))
  (bind _returnvalue_2 (`KismetMathLibrary.MakeVector` (.x (`self.K2_GetActorLocation` (`self.Player`))) (.y (`self.K2_GetActorLocation` (`self.Player`)))))
  (bind _returnvalue_3 (`KismetMathLibrary.MakeVector` (.x (`self.K2_GetActorLocation` (`self.Player`))) (.y (`self.K2_GetActorLocation` (`self.Player`)))))
  (bind _returnvalue_4 (`KismetMathLibrary.MakeVector` (.x (`self.K2_GetActorLocation` (`self.Player`))) (.y (`self.K2_GetActorLocation` (`self.Player`)))))
  (`|ExecutionSequence`
    (:`then_0`
      (set `local.DistRight` 99999.0)
      (set `local.DistLeft` 99999.0)
      (set `local.DistUp` 99999.0)
      (set `local.DistDown` 99999.0))
    (:`then_1`
      (set `local.R` null)
      (set `local.L` null)
      (set `local.U` null)
      (set `local.D` null)
      (`|ExecutionSequence`
        (:`then_0`
          (bind _outhits (`KismetSystemLibrary.SphereTraceMultiForObjects` :`Start` _returnvalue_2 :`End` (+ _returnvalue_2 (* (`KismetMathLibrary.GetRightVector` (`self.K2_GetActorRotation` (`self.Cam`))) 5000.0)) :`Radius` 10.0 :`ObjectTypes` (`|MakeArray` "ObjectTypeQuery2" :!type "EObjectTypeQuery Enum") :`DrawDebugType` "ForDuration"))
          (for _array_element _outhits
            (bind _asbp_spline_point_collision (cast `/Game/Blueprints/Assets/BP_SplinePointCollision` (`.HitActor` (`GameplayStatics.BreakHitResult` _array_element))))
            (bind _returnvalue_5 (`self.GetDistanceTo` _asbp_spline_point_collision (`self.Player`)))
            (if (and (< _returnvalue_5 (`local.DistRight`)) (`KismetArrayLibrary.Array_Contains` Splines (`/Game/Blueprints/Assets/BP_SplinePointCollision.Spline` _asbp_spline_point_collision)) (== (`KismetArrayLibrary.Array_Contains` CurrentPoints _asbp_spline_point_collision) false))
              (set `local.R` _asbp_spline_point_collision)
              (set `local.DistRight` _returnvalue_5))))
        (:`then_1`
          (bind _outhits_2 (`KismetSystemLibrary.SphereTraceMultiForObjects` :`Start` _returnvalue_3 :`End` (+ _returnvalue_3 (* (`KismetMathLibrary.GetRightVector` (`self.K2_GetActorRotation` (`self.Cam`))) -5000.0)) :`Radius` 10.0 :`ObjectTypes` (`|MakeArray` "ObjectTypeQuery2" :!type "EObjectTypeQuery Enum") :`DrawDebugType` "ForDuration"))
          (for _array_element_2 _outhits_2
            (bind _asbp_spline_point_collision_2 (cast `/Game/Blueprints/Assets/BP_SplinePointCollision` (`.HitActor` (`GameplayStatics.BreakHitResult` _array_element_2))))
            (bind _returnvalue_6 (`self.GetDistanceTo` _asbp_spline_point_collision_2 (`self.Player`)))
            (if (and (< _returnvalue_6 (`local.DistLeft`)) (`KismetArrayLibrary.Array_Contains` Splines (`/Game/Blueprints/Assets/BP_SplinePointCollision.Spline` _asbp_spline_point_collision_2)) (== (`KismetArrayLibrary.Array_Contains` CurrentPoints _asbp_spline_point_collision_2) false))
              (set `local.L` _asbp_spline_point_collision_2)
              (set `local.DistLeft` _returnvalue_6))))
        (:`then_2`
          (bind _outhits_3 (`KismetSystemLibrary.SphereTraceMultiForObjects` :`Start` _returnvalue_4 :`End` (+ _returnvalue_4 (* (`KismetMathLibrary.MakeVector` (.x (`KismetMathLibrary.GetForwardVector` (`self.K2_GetActorRotation` (`self.Cam`)))) (.y (`KismetMathLibrary.GetForwardVector` (`self.K2_GetActorRotation` (`self.Cam`))))) 5000.0)) :`Radius` 10.0 :`ObjectTypes` (`|MakeArray` "ObjectTypeQuery2" :!type "EObjectTypeQuery Enum") :`DrawDebugType` "ForDuration"))
          (for _array_element_3 _outhits_3
            (bind _asbp_spline_point_collision_3 (cast `/Game/Blueprints/Assets/BP_SplinePointCollision` (`.HitActor` (`GameplayStatics.BreakHitResult` _array_element_3))))
            (bind _returnvalue_7 (`self.GetDistanceTo` _asbp_spline_point_collision_3 (`self.Player`)))
            (if (and (< _returnvalue_7 (`local.DistUp`)) (`KismetArrayLibrary.Array_Contains` Splines (`/Game/Blueprints/Assets/BP_SplinePointCollision.Spline` _asbp_spline_point_collision_3)) (== (`KismetArrayLibrary.Array_Contains` CurrentPoints _asbp_spline_point_collision_3) false))
              (set `local.U` _asbp_spline_point_collision_3)
              (set `local.DistUp` _returnvalue_7))))
        (:`then_3`
          (bind _outhits_4 (`KismetSystemLibrary.SphereTraceMultiForObjects` :`Start` _returnvalue :`End` (+ _returnvalue (* (`KismetMathLibrary.MakeVector` (.x (`KismetMathLibrary.GetForwardVector` (`self.K2_GetActorRotation` (`self.Cam`)))) (.y (`KismetMathLibrary.GetForwardVector` (`self.K2_GetActorRotation` (`self.Cam`))))) -5000.0)) :`Radius` 10.0 :`ObjectTypes` (`|MakeArray` "ObjectTypeQuery2" :!type "EObjectTypeQuery Enum") :`DrawDebugType` "ForDuration"))
          (for _array_element_4 _outhits_4
            (bind _asbp_spline_point_collision_4 (cast `/Game/Blueprints/Assets/BP_SplinePointCollision` (`.HitActor` (`GameplayStatics.BreakHitResult` _array_element_4))))
            (bind _returnvalue_8 (`self.GetDistanceTo` _asbp_spline_point_collision_4 (`self.Player`)))
            (if (and (< _returnvalue_8 (`local.DistDown`)) (`KismetArrayLibrary.Array_Contains` Splines (`/Game/Blueprints/Assets/BP_SplinePointCollision.Spline` _asbp_spline_point_collision_4)) (== (`KismetArrayLibrary.Array_Contains` CurrentPoints _asbp_spline_point_collision_4) false))
              (set `local.D` _asbp_spline_point_collision_4)
              (set `local.DistDown` _returnvalue_8))))
        (:`then_4`
          (return (`local.R`) (`local.L`) (`local.U`) (`local.D`)))))))

(fn `Instantiate spline point collision`
  (params (Transform :type "Transform Structure") (Spline :type "/Game/Blueprints/Assets/BP_Spline Object Reference") (Indice :type Integer))
  (bind _returnvalue (`|SpawnActorFromClass` "/Game/Blueprints/Assets/BP_SplinePointCollision.BP_SplinePointCollision_C" Transform "AlwaysSpawn" "MultiplyWithRoot" null null))
  (set `/Game/Blueprints/Assets/BP_SplinePointCollision.Spline` Spline _returnvalue)
  (set `/Game/Blueprints/Assets/BP_SplinePointCollision.Indice` Indice _returnvalue)
  (return))

(fn `ToMove`
  (bind (_currentpoints _splines) (`self.GetCurrentPoints`))
  (bind (_right _left _up _down) (`self.GetNextPoints` _currentpoints _splines))
  (`|ExecutionSequence`
    (:`then_0`
      (`self.Create Arrows` _right _left _up _down))
    (:`then_1`
      (set `self.RightPoint` _right))
    (:`then_2`
      (set `self.LeftPoint` _left))
    (:`then_3`
      (set `self.UpPoint` _up))
    (:`then_4`
      (set `self.DownPoint` _down))
    (:`then_5`
      (set `self.Current Points` _currentpoints))))

(fn `UserConstructionScript`)
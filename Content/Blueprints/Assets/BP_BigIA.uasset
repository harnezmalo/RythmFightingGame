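; BP_BigIA is a rotating sentinel AI that checks whether it can see the player.
; A looping Rotation timeline drives its yaw continuously from BeginPlay.
; Each tick it line-traces toward BP_Player, ignoring arrows, then uses a dot-product test against its forward vector as a view cone.
; The result sets the GameManager's UITest state text to "Dead" when the player is seen, otherwise "Alive".
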(event `self.ReceiveBeginPlay`
  (bind _returnvalue (`GameplayStatics.GetActorOfClass` "/Game/Blueprints/Contrôlables/BP_Player.BP_Player_C"))
  (set `self.Player` _returnvalue)
  (`self.Rotate`)
  (bind _returnvalue_2 (`GameplayStatics.GetActorOfClass` "/Game/Blueprints/Assets/BP_GameManager.BP_GameManager_C"))
  (set `self.GameManager` _returnvalue_2))

(event `self.ReceiveTick`
  (params (DeltaSeconds :type "Float (single-precision)"))
  (bind _returnvalue (`self.K2_GetActorLocation`))
  (bind _ui_test (`/Game/Blueprints/Assets/BP_GameManager.UI_Test` (`self.GameManager`)))
  (bind _outactors (`GameplayStatics.GetAllActorsOfClass` "/Game/Blueprints/Assets/BP_Arrow.BP_Arrow_C"))
  (bind _outhit (`KismetSystemLibrary.LineTraceSingle` _returnvalue (+ _returnvalue (* (`KismetMathLibrary.Normal` (- (`self.K2_GetActorLocation` (`self.Player`)) _returnvalue)) (9999.0 9999.0 9999.0))) "TraceTypeQuery2" false _outactors "ForOneFrame"))
  (cast `/Game/Blueprints/Contrôlables/BP_Player` (`.HitActor` (`GameplayStatics.BreakHitResult` _outhit))
    (:`then`
      (if (>= (`KismetMathLibrary.Dot_VectorVector` (`SceneComponent.GetForwardVector` (`self.CapsuleComponent`)) (`KismetMathLibrary.Normal` (- (`self.K2_GetActorLocation` (`self.Player`)) (`self.K2_GetActorLocation`)))) 0.8)
        (set `/Game/Blueprints/UI/WB_TestState.State` (`|FormatText` "Dead") _ui_test)
        (else
          (set `/Game/Blueprints/UI/WB_TestState.State` (`|FormatText` "Alive") _ui_test :!label _label))))
    (:`CastFailed`
      (goto _label))))

(event `Rotate`
  (bind (_direction _rot) (`Timeline|Rotation` :!via `PlayFromStart`)
    (:`Update`
      (`self.K2_SetActorRotation` (`KismetMathLibrary.MakeRotator` 0.0 0.0 _rot)))
    (:`Finished`
      (`self.Rotate`))))

(fn `UserConstructionScript`)